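; Base networked 2D enemy that deals contact damage to players and chases whoever hurts it.
; Server-side overlap with tagged players runs a looping timer that damages overlapping, non-god players using AnimalInfo stats.
; Taking damage lowers health, pauses movement for the flipbook's length, stops AI logic, then loops moves to the attacker and a short horizontal offset.
; Replicated movement state selects idle, move or hit flipbooks through OnRep.
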(event OnComponentBeginOverlap(Collision)
  (params (OverlappedComponent :type Primitive%20Component%20Object%20Reference) (OtherActor :type Actor%20Object%20Reference) (OtherComp :type Primitive%20Component%20Object%20Reference) (OtherBodyIndex :type Integer) (bFromSweep :type Boolean) (SweepResult :type Hit%20Result%20Structure%20%28by%20ref%29))
  (Networking|SwitchHasAuthority
    (:Authority
      (if (Actor|ActorHasTag OtherActor "Player")
        (CallFunction|StartApplyDamage true)))))

(event OnComponentEndOverlap(Collision)
  (params (OverlappedComponent :type Primitive%20Component%20Object%20Reference) (OtherActor :type Actor%20Object%20Reference) (OtherComp :type Primitive%20Component%20Object%20Reference) (OtherBodyIndex :type Integer))
  (Networking|SwitchHasAuthority
    (:Authority
      (if (Actor|ActorHasTag OtherActor "Player")
        (CallFunction|StartApplyDamage false)))))

(event Custom|SRV_setMovementState
  (params (Movement%20State :type E_MovementState%20Enum :default "NewEnumerator0"))
  (Variables|Default|SetMovementState Movement%20State))

(event Custom|SRV_StartApplyDamage
  (params (bApplyDamage :type Boolean))
  (if bApplyDamage
    (bind _returnvalue (Utilities|Time|SetTimerbyEvent (delegate Custom|ApplyDamage) 0.1 true))
    (Variables|Default|SetApplyDamageHandle _returnvalue)
    (else
      (Utilities|Time|ClearandInvalidateTimerbyHandle (Variables|Default|GetApplyDamageHandle)))))

(event Custom|ApplyDamage
  (for _array_element (Collision|GetOverlappingActors "/Game/Blueprints/Player/BP_PlayerBase.BP_PlayerBase_C" :!class /Script/Engine.Actor)
    (bind _player (Class|INTPlayerBase|GetPlayerRef(Message) _array_element))
    (if (not (Variables|/Game/Blueprints/Player/BP_PlayerBase.BP_PlayerBase_C|GetIsGod _player))
      (Game|Damage|ApplyDamage _player (.Damage (Utilities|Struct|BreakST_AnimalInfo (Variables|Default|GetAnimalInfo))) (Pawn|GetController) 0 "/Script/Engine.DamageType"))))

(event EventSetMovementState
  (params (Movement%20State :type E_MovementState%20Enum :default "NewEnumerator0"))
  (CallFunction|SRVSetMovementState Movement%20State))

(event Game|Damage|EventAnyDamage
  (params (Damage :type Float%20%28single-precision%29) (DamageType :type Damage%20Type%20Object%20Reference) (InstigatedBy :type Controller%20Object%20Reference) (DamageCauser :type Actor%20Object%20Reference))
  (bind _returnvalue (Transformation|GetActorLocation))
  (bind (_x _y _z) (Math|Vector|BreakVector _returnvalue))
  (Variables|Default|SetPlayerContorller InstigatedBy)
  (CallFunction|SetMovementState "NewEnumerator7")
  (Pawn|Components|CharacterMovement|SetMovementMode (Variables|Character|GetCharacterMovement) "MOVE_None" 0)
  (bind _structout (Utilities|Struct|SetmembersinST_AnimalInfo (Variables|Default|GetAnimalInfo) (Math|Float|Clamp(Float) (- (.Health (Utilities|Struct|BreakST_AnimalInfo (Variables|Default|GetAnimalInfo))) Damage) 0.0 (.Health (Utilities|Struct|BreakST_AnimalInfo (Variables|Default|GetAnimalInfo))))))
  (Development|PrintString (Utilities|String|ToString(Float) (Math|Float|Clamp(Float) (- (.Health (Utilities|Struct|BreakST_AnimalInfo (Variables|Default|GetAnimalInfo))) Damage) 0.0 (.Health (Utilities|Struct|BreakST_AnimalInfo (Variables|Default|GetAnimalInfo))))))
  (Variables|Default|SetAnimalInfo _structout)
  (Utilities|FlowControl|Delay (Class|PaperFlipbookComponent|GetFlipbookLength (Variables|Default|GetSprite)))
  (Components|Movement|StopMovementImmediately (Variables|Character|GetCharacterMovement))
  (bind _aicontroller (Class|INTAIController|GetAIControllerRef(Message) (Pawn|GetController)))
  (AI|Logic|StopLogic (Variables|/Script/AIModule.AIController|GetBrainComponent _aicontroller) "Hit")
  (Pawn|Components|CharacterMovement|SetMovementMode (Variables|Character|GetCharacterMovement) "MOVE_Walking" 0)
  (CallFunction|SetMovementState "NewEnumerator2")
  (AI|AIMoveTo self (Transformation|GetActorLocation (Pawn|GetControlledPawn (Variables|Default|GetPlayerContorller))) (Pawn|GetControlledPawn (Variables|Default|GetPlayerContorller)) 2.0 false :!label _label
    (:OnSuccess
      (AI|AIMoveTo (AI|GetAIController self) (Math|Vector|MakeVector (+ _x (Math|Float|SelectFloat -125.0 125.0 (< (.X (Math|Vector|BreakVector (Transformation|GetActorLocation (Pawn|GetControlledPawn (Variables|Default|GetPlayerContorller))))) _x))) _y _z) 0 -1.0 "Default" "Default" true true
        (:OnMoveFinished
          (goto _label))))))

(event EventStartApplyDamage
  (params (bApplyDamage :type Boolean))
  (CallFunction|SRVStartApplyDamage bApplyDamage))

(fn ConstructionScript
  (|CallParentFunction))

(fn OnRepBIsMoving
  (bind _sprite (Variables|Default|GetSprite))
  (bind _animalinfo (Variables|Default|GetAnimalInfo))
  (bind (_idleanimation _moveanimation) (Utilities|Struct|BreakST_AnimalInfo _animalinfo))
  (if (not (Variables|Default|GetbIsMoving))
    (Sprite|SetFlipbook _sprite _idleanimation)
    (else
      (Sprite|SetFlipbook _sprite _moveanimation))))

(fn OnRepMovementState
  (bind _sprite (Variables|Default|GetSprite))
  (bind _animalinfo (Variables|Default|GetAnimalInfo))
  (bind (_idleanimation _moveanimation _hitanimation) (Utilities|Struct|BreakST_AnimalInfo _animalinfo))
  (switch Utilities|FlowControl|Switch|SwitchonE_MovementState (Variables|Default|GetMovementState)
    (:NewEnumerator0
      (Sprite|SetFlipbook _sprite _idleanimation))
    (:NewEnumerator2
      (Sprite|SetFlipbook _sprite _moveanimation))
    (:NewEnumerator7
      (Sprite|SetFlipbook _sprite _hitanimation))))

(fn OnRepPlayerContorller)

(fn GetEnemyRef
  (return self))