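; Player controller for a MapleStory-style game that handles character selection, pawn possession and the player's UI.
; Client events create the character selection and main widgets, showing only selection at start, and forward enemy name and health percent to the main widget.
; Character choice passes through a server event to the game mode via interface message.
; A separate SpawnPlayer event spawns and possesses the chosen character.
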(event Custom|CL_UpdateHealthBar
  (params (Percent :type Float%20%28single-precision%29) (EnemyName :type String))
  (Default|UpdateHealth (Variables|Default|GetWB_Main) Percent EnemyName))

(event Custom|CL_InitializeWidgets
  (bind _returnvalue (UserInterface|CreateWidget "/Game/UI/WB_CharacterSelection.WB_CharacterSelection_C"))
  (bind _output_get (Variables|Default|SetWB_CharacterSelection _returnvalue))
  (UserInterface|Viewport|AddtoViewport _output_get 0)
  (bind _returnvalue_2 (UserInterface|CreateWidget "/Game/UI/WB_Main.WB_Main_C"))
  (Variables|Default|SetWB_Main _returnvalue_2))

(event Custom|SRV_SelectCharacter
  (params (Player :type Actor%20Class%20Reference) (Location :type Vector))
  (bind _gamemode (Class|INTGameMode|GetGameModeRef(Message) (Game|GetGameMode)))
  (Class|INTGameMode|RequestSpawnPlayer(Message) _gamemode self Player Location))

(event EventBeginPlay
  (CallFunction|InitializeWidgets))

(event EventInitializeWidgets
  (CallFunction|CLInitializeWidgets))

(event EventSelectCharacter
  (params (Player :type Actor%20Class%20Reference) (SpawnLocatrion :type Vector :default "0, 0, 0"))
  (CallFunction|SRVSelectCharacter Player SpawnLocatrion))

(event EventSpawnPlayer
  (params (Player :type Actor%20Class%20Reference) (SpawnTransform :type Transform))
  (bind _returnvalue (Game|SpawnActorfromClass Player SpawnTransform "AdjustIfPossibleButAlwaysSpawn" "MultiplyWithRoot" 0 0))
  (bind _player (Class|INTPlayerBase|GetPlayerRef(Message) _returnvalue))
  (Pawn|Possess _player))

(event EventUpdateHealthBar
  (params (Percent :type Float%20%28double-precision%29) (EnemyName :type String))
  (CallFunction|CLUpdateHealthBar Percent EnemyName))

(fn ConstructionScript)

(fn GetPlayerControllerRef
  (return self))